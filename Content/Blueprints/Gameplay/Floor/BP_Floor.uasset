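; BP_Floor is a floor actor that tints its mesh to match the current difficulty level.
; On BeginPlay it creates a dynamic instance of MM_Floor_Inst and reads DifficultyLevel from BP_GameInstance.
; Each of the three levels sets its own Color parameter before the material is applied to the mesh.
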(event `self.ReceiveBeginPlay`
  (bind _returnvalue (`PrimitiveComponent.CreateDynamicMaterialInstance` (`self.StaticMeshComponent`) 0 "/Game/Blueprints/Gameplay/Floor/MM_Floor_Inst.MM_Floor_Inst" "None"))
  (set `self.DynMaterial` _returnvalue)
  (bind _asbp_game_instance (cast `/Game/Blueprints/GameInstance/BP_GameInstance` (`GameplayStatics.GetGameInstance`)))
  (`/Engine/EditorBlueprintResources/StandardMacros.IsValid` _asbp_game_instance
    (:`Is Valid`
      (switch `int` (`KulkiGameInstance.DifficultyLevel` _asbp_game_instance)
        (:`1`
          (`MaterialInstanceDynamic.SetVectorParameterValue` (`self.DynMaterial`) "Color" (struct :`R` 0.014444 :`G` 0.030713 :`B` 0.030713 :`A` 1.0)))
        (:`2`
          (`MaterialInstanceDynamic.SetVectorParameterValue` (`self.DynMaterial`) "Color" (struct :`R` 0.453125 :`G` 0.157112 :`B` 0.104313 :`A` 1.0)))
        (:`3`
          (`MaterialInstanceDynamic.SetVectorParameterValue` (`self.DynMaterial`) "Color" (struct :`R` 0.169735 :`G` 0.124626 :`B` 0.419792 :`A` 1.0))))
      (`PrimitiveComponent.SetMaterial` (`self.StaticMeshComponent`) 0 (`self.DynMaterial`)))))

(fn `UserConstructionScript`)