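; BP_Floor is a floor actor whose overlay color reflects the game's current difficulty level.
; On BeginPlay it creates a dynamic instance of the static mesh's overlay material and reads DifficultyLevel from BP_GameInstance.
; Each of the three levels sets a different Color parameter, then the instance is reapplied as the mesh's overlay material.
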(event `self.ReceiveBeginPlay`
  (bind _returnvalue (`KismetMaterialLibrary.CreateDynamicMaterialInstance` (`MeshComponent.GetOverlayMaterial` (`self.StaticMeshComponent`))))
  (set `self.DynMaterial` _returnvalue)
  (bind _asbp_game_instance (cast `/Game/Blueprints/GameInstance/BP_GameInstance` (`GameplayStatics.GetGameInstance`)))
  (`/Engine/EditorBlueprintResources/StandardMacros.IsValid` _asbp_game_instance
    (:`Is Valid`
      (switch `int` (`KulkiGameInstance.DifficultyLevel` _asbp_game_instance)
        (:`1`
          (`MaterialInstanceDynamic.SetVectorParameterValue` (`self.DynMaterial`) "Color" (struct :`R` 0.311588 :`G` 1.0 :`B` 0.966164 :`A` 1.0)))
        (:`2`
          (`MaterialInstanceDynamic.SetVectorParameterValue` (`self.DynMaterial`) "Color" (struct :`R` 1.0 :`G` 0.151367 :`A` 1.0)))
        (:`3`
          (`MaterialInstanceDynamic.SetVectorParameterValue` (`self.DynMaterial`) "Color" (struct :`R` 0.152826 :`B` 1.0 :`A` 1.0))))
      (`MeshComponent.SetOverlayMaterial` (`self.StaticMeshComponent`) (`self.DynMaterial`)))))

(fn `UserConstructionScript`)